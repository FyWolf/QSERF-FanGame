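; BatteryLight is a ship battery status indicator that shows a colored point light and matching indicator material.
; Three signal events toggle it on or off in red for battery down, orange for battery low and green for interaction.
; BatteryDead clears CanWork, which blocks those events and makes Tick force the light off.
; While lit, Tick also calls BatteryUpdate on the Ship every frame with a small fixed amount, independent of delta time.
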(event `self.BatteryDown`
  (params (Signal :type Boolean))
  (bind _pointlight (`self.PointLight`))
  (bind _indicator (`self.indicator`))
  (if (`self.CanWork`)
    (`SceneComponent.SetVisibility` _pointlight Signal false)
    (`LightComponent.SetLightColor` _pointlight (struct :`R` 1.0 :`A` 1.0) true)
    (if Signal
      (`PrimitiveComponent.SetMaterial` _indicator 1 "/Game/Materials/IndicatorLightOn-red.IndicatorLightOn-red")
      (set `self.IsOn` true)
      (else
        (`PrimitiveComponent.SetMaterial` _indicator 1 "/Game/Materials/IndicatorLightOff.IndicatorLightOff")
        (set `self.IsOn` false)))))

(event `self.BatteryLow`
  (params (Signal :type Boolean))
  (bind _pointlight (`self.PointLight`))
  (bind _indicator (`self.indicator`))
  (if (`self.CanWork`)
    (`SceneComponent.SetVisibility` _pointlight Signal false)
    (`LightComponent.SetLightColor` _pointlight (struct :`R` 1.0 :`G` 0.224 :`A` 1.0) true)
    (if Signal
      (`PrimitiveComponent.SetMaterial` _indicator 1 "/Game/Materials/IndicatorLightOn-orange.IndicatorLightOn-orange")
      (set `self.IsOn` true)
      (else
        (`PrimitiveComponent.SetMaterial` _indicator 1 "/Game/Materials/IndicatorLightOff.IndicatorLightOff")
        (set `self.IsOn` false)))))

(event `self.On Interraction`
  (params (BoolSignal :type Boolean))
  (bind _pointlight (`self.PointLight`))
  (bind _indicator (`self.indicator`))
  (if (`self.CanWork`)
    (`SceneComponent.SetVisibility` _pointlight BoolSignal false)
    (`LightComponent.SetLightColor` _pointlight (struct :`G` 1.0 :`A` 1.0) true)
    (if BoolSignal
      (`PrimitiveComponent.SetMaterial` _indicator 1 "/Game/Materials/IndicatorLightOn-green.IndicatorLightOn-green")
      (set `self.IsOn` true)
      (else
        (`PrimitiveComponent.SetMaterial` _indicator 1 "/Game/Materials/IndicatorLightOff.IndicatorLightOff")
        (set `self.IsOn` false)))))

(event `self.ReceiveTick`
  (params (DeltaSeconds :type "Float (single-precision)"))
  (`|ExecutionSequence`
    (:`then_0`
      (if (not (`self.CanWork`))
        (`SceneComponent.SetVisibility` (`self.PointLight`) false false)
        (`PrimitiveComponent.SetMaterial` (`self.indicator`) 1 "/Game/Materials/IndicatorLightOff.IndicatorLightOff")
        (set `self.IsOn` false)))
    (:`then_1`
      (if (`self.IsOn`)
        (`/Game/blueprints/Cockpit.BatteryUpdate` (`self.Ship`) 0.001)))))

(event `self.BatteryDead`
  (params (IsBatteryDead :type Boolean))
  (set `self.CanWork` (not IsBatteryDead)))

(fn `UserConstructionScript`
  (`parent.UserConstructionScript`))