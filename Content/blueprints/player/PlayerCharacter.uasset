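; First-person player character with movement, jump, hold-to-zoom, timeline-driven crouch and a HUD widget.
; Camera line traces on Tick outline batteries via custom depth, detect slots while carrying one, and flag ActorMaster targets on the HUD for E.
; A picks up, drops or slots batteries, registering slotted ones with RessourcesComponent; held ones follow HoldingPlace.
; Interact holds Button_Master buttons, with a delay loop releasing them when the player moves out of range.
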(event `Key|RightMouseButton`
  (params (Key :type "Key Structure"))
  (bind _camera (`self.Camera`))
  ;[1 1 0] Zoom
  (:`Pressed`
    (`CameraComponent.SetFieldOfView` _camera 30.0))
  (:`Released`
    (`CameraComponent.SetFieldOfView` _camera 90.0)))

(event `InputAxis|Move Right`
  (params (AxisValue :type "Float (single-precision)"))
  ;[1 1 0] Movement code
  (`self.AddMovementInput` (`KismetMathLibrary.GetRightVector` (`KismetMathLibrary.MakeRotator` 0.0 0.0 (.yaw (`self.GetControlRotation`)))) AxisValue))

(event `InputAxis|Move Forward`
  (params (AxisValue :type "Float (single-precision)"))
  ;[1 1 0] Movement code
  (`self.AddMovementInput` (`KismetMathLibrary.GetForwardVector` (`KismetMathLibrary.MakeRotator` 0.0 0.0 (.yaw (`self.GetControlRotation`)))) AxisValue))

(event `InputAxis|lookright`
  (params (AxisValue :type "Float (single-precision)"))
  ;[1 1 0] Movement code
  (`self.AddControllerYawInput` AxisValue))

(event `InputAction|Jump`
  (params (Key :type "Key Structure"))
  ;[1 1 0] Movement code
  (:`Pressed`
    (`self.Jump`))
  (:`Released`
    (`self.StopJumping`)))

(event `self.ReceiveBeginPlay`
  ;[1 0 1] Start code (hud display for crosshair)
  (bind _returnvalue (`|CreateWidget` "/Game/blueprints/player/hud.hud_C"))
  (set `self.ReferenceHUD` _returnvalue)
  (`UserWidget.AddToViewport` _returnvalue 0))

(event `InputAxis|lookup`
  (params (AxisValue :type "Float (single-precision)"))
  ;[1 1 0] Movement code
  (`self.AddControllerPitchInput` AxisValue))

(event `InputAction|Interract`
  (params (Key :type "Key Structure"))
  (bind _camera (`self.Camera`))
  (bind _returnvalue (`SceneComponent.K2_GetComponentLocation` _camera))
  ;[1 1 0] Interraction code
  (:`Pressed`
    (bind _outhit (`KismetSystemLibrary.LineTraceSingle` _returnvalue (+ _returnvalue (* (`SceneComponent.GetForwardVector` _camera) 250.0)) "TraceTypeQuery2"))
    (bind (_bblockinghit _binitialoverlap _time _distance _location _impactpoint _normal _impactnormal _physmat _hitactor) (`GameplayStatics.BreakHitResult` _outhit))
    (if _bblockinghit
      (set `self.Hit Actor` _hitactor)
      (bind _asbutton_master (cast `/Game/blueprints/Button_Master` _hitactor))
      (`/Game/blueprints/Button_Master.PushOn` _asbutton_master)
      (`self.CheckDistance`)))
  (:`Released`
    (bind _asbutton_master_2 (cast `/Game/blueprints/Button_Master` (`self.Hit Actor`) :!label _label))
    (`/Game/blueprints/Button_Master.PushOff` _asbutton_master_2)))

(event `self.ReceiveTick`
  (params (DeltaSeconds :type "Float (single-precision)"))
  (bind _camera (`self.Camera`))
  (bind _referencehud (`self.ReferenceHUD`))
  (bind _camera_2 (`self.Camera`))
  (bind _battery (`self.Battery`))
  (bind _returnvalue (`SceneComponent.K2_GetComponentLocation` _camera_2))
  (bind _returnvalue_2 (`SceneComponent.K2_GetComponentLocation` _camera))
  (`|ExecutionSequence`
    (:`then_0`
      (if (`self.IsHolding`)
        (`self.K2_SetActorLocation` _battery (`SceneComponent.K2_GetComponentLocation` (`self.HoldingPlace`)) false true)
        (`self.K2_SetActorRotation` _battery (`SceneComponent.K2_GetComponentRotation` (`self.HoldingPlace`)) false)))
    (:`then_1`
      (bind _outhit (`KismetSystemLibrary.LineTraceSingle` _returnvalue_2 (+ _returnvalue_2 (* (`SceneComponent.GetForwardVector` _camera) 250.0)) "TraceTypeQuery2"))
      (if (`self.IsHolding`)
        (bind (_bblockinghit _binitialoverlap _time _distance _location _impactpoint _normal _impactnormal _physmat _hitactor) (`GameplayStatics.BreakHitResult` _outhit))
        (bind _returnvalue_3 (`GameplayStatics.GetObjectClass` _hitactor))
        (if (== _returnvalue_3 "/Game/blueprints/BatterySlot.BatterySlot_C")
          (`|ExecutionSequence`
            (:`then_0`
              (`/Engine/EditorBlueprintResources/StandardMacros.DoOnce` false :!label _label_2
                (:`Completed`
                  (bind _asbattery_slot (cast `/Game/blueprints/BatterySlot` _hitactor))
                  (if (not (`/Game/blueprints/BatterySlot.BatterySlotOccupied` _asbattery_slot))
                    (set `self.BatterySlot` _asbattery_slot)
                    (`/Game/blueprints/BatterySlot.BeginOverlap` _asbattery_slot)
                    (set `self.LookingAtSlot` true)))))
            (:`then_1`
              (goto _label_3 :!via `Reset`)))
          (else
            (`|ExecutionSequence`
              (:`then_0`
                (goto _label_2 :!via `Reset`))
              (:`then_1`
                (`/Engine/EditorBlueprintResources/StandardMacros.DoOnce` false :!label _label_3
                  (:`Completed`
                    (bind _asbattery_slot_2 (cast `/Game/blueprints/BatterySlot` (`self.BatterySlot`)))
                    (if (not (`/Game/blueprints/BatterySlot.BatterySlotOccupied` _asbattery_slot_2))
                      (set `self.BatterySlot` null)
                      (`/Game/blueprints/BatterySlot.EndOverlap` _asbattery_slot_2)
                      (set `self.LookingAtSlot` false))))))))
        (elif (== _returnvalue_3 "/Game/blueprints/Battery.Battery_C")
          (set `self.Battery` _hitactor)
          (if (== _hitactor (`self.Battery`))
            (`|ExecutionSequence`
              (:`then_0`
                (`/Engine/EditorBlueprintResources/StandardMacros.DoOnce` false :!label _label_4
                  (:`Completed`
                    (bind _asbattery (cast `/Game/blueprints/Battery` _hitactor))
                    (bind _battery_2 (`/Game/blueprints/Battery.battery` _asbattery))
                    (`PrimitiveComponent.SetRenderCustomDepth` _battery_2 true)
                    (`PrimitiveComponent.SetCustomDepthStencilValue` _battery_2 0)
                    (set `self.lookingAtBattery` true))))
              (:`then_1`
                (goto _label_6 :!via `Reset`)))
            (else
              (`|ExecutionSequence` :!label _label_5
                (:`then_0`
                  (goto _label_4 :!via `Reset`))
                (:`then_1`
                  (`/Engine/EditorBlueprintResources/StandardMacros.DoOnce` false :!label _label_6
                    (:`Completed`
                      (bind _asbattery_2 (cast `/Game/blueprints/Battery` (`self.Battery`)))
                      (set `self.Battery` null)
                      (bind _battery_3 (`/Game/blueprints/Battery.battery` _asbattery_2))
                      (`PrimitiveComponent.SetRenderCustomDepth` _battery_3 false)
                      (`PrimitiveComponent.SetCustomDepthStencilValue` _battery_3 0)
                      (set `self.lookingAtBattery` false)))))))
          (else
            (goto _label_5)))))
    (:`then_2`
      (bind _outhit_2 (`KismetSystemLibrary.LineTraceSingle` _returnvalue (+ _returnvalue (* (`SceneComponent.GetForwardVector` _camera_2) 350.0)) "TraceTypeQuery2" true))
      (bind (_bblockinghit_2 _binitialoverlap_2 _time_2 _distance_2 _location_2 _impactpoint_2 _normal_2 _impactnormal_2 _physmat_2 _hitactor_2) (`GameplayStatics.BreakHitResult` _outhit_2))
      (if (`KismetMathLibrary.ClassIsChildOf` (`GameplayStatics.GetObjectClass` _hitactor_2) "/Game/blueprints/ActorMaster.ActorMaster_C")
        (set `/Game/blueprints/player/hud.ActionAvailable?` true _referencehud)
        (set `self.InterractionAvailable?` true)
        (set `self.ActorInSight` _hitactor_2)
        (else
          (set `/Game/blueprints/player/hud.ActionAvailable?` false _referencehud)
          (set `self.InterractionAvailable?` false)
          (set `self.ActorInSight` null))))))

(event `CheckDistance`
  ;[1 1 0] Interraction code
  ;;[1 1 1] Check distance between button and player
  (if (< (`self.GetDistanceTo` (`self.Hit Actor`) self) 250.0) :!label _label_7
    (`KismetSystemLibrary.Delay` 0.01)
    (goto _label_7)
    (else
      (goto _label))))

(event `Key|E`
  (params (Key :type "Key Structure"))
  (:`Pressed`
    (if (`self.InterractionAvailable?`)
      (bind _asactor_master (cast `/Game/blueprints/ActorMaster` (`self.ActorInSight`)))
      (`/Game/blueprints/ActorMaster.ActionLaunched` _asactor_master false))))

(event `Key|A`
  (params (Key :type "Key Structure"))
  (bind _batteryslot (`self.BatterySlot`))
  (bind _battery (`self.Battery`))
  (bind _asbattery (cast `/Game/blueprints/Battery` _battery :!pure true))
  (bind _rootcomponent (`Actor.RootComponent` (`self.BatterySlot`)))
  (bind _battery_2 (`/Game/blueprints/Battery.battery` _asbattery))
  (bind _battery_3 (`/Game/blueprints/Battery.battery` _asbattery))
  ;[1 0 1] Pickup and place system
  (:`Pressed`
    (if (`KismetSystemLibrary.IsValid` _battery)
      (if (`self.IsHolding`)
        (if (`self.LookingAtSlot`)
          (bind _asbattery_slot (cast `/Game/blueprints/BatterySlot` (`self.BatterySlot`)))
          (if (not (`/Game/blueprints/BatterySlot.BatterySlotOccupied` _asbattery_slot))
            (set `self.IsHolding` false)
            (`self.K2_SetActorLocationAndRotation` (`self.Battery`) (`SceneComponent.K2_GetComponentLocation` _rootcomponent) (`SceneComponent.K2_GetComponentRotation` _rootcomponent) false true)
            (set `/Game/blueprints/Battery.SlotID` _batteryslot _asbattery)
            (set `/Game/blueprints/Battery.IsPluggedIn` true _asbattery)
            (`/Game/blueprints/Battery.BatteryPlugged` _asbattery)
            (`/Game/blueprints/Ressources_Component.ConnectBattery` (`self.Ressources_Component`) _asbattery)
            (bind _asbattery_slot_2 (cast `/Game/blueprints/BatterySlot` _batteryslot))
            (`/Game/blueprints/BatterySlot.EndOverlap` _asbattery_slot_2)
            (set `/Game/blueprints/BatterySlot.ConnectedBattery` _asbattery _asbattery_slot_2)
            (set `/Game/blueprints/BatterySlot.BatterySlotOccupied` true _asbattery_slot_2)
            (set `self.Battery` null))
          (else
            (set `self.IsHolding` false)
            (`PrimitiveComponent.SetSimulatePhysics` (`/Game/blueprints/Battery.battery` _asbattery) true)
            (set `self.Battery` null)))
        (elif (`/Game/blueprints/Battery.IsPluggedIn` _asbattery)
          (set `/Game/blueprints/Battery.IsPluggedIn` false _asbattery)
          (bind _asbattery_slot_3 (cast `/Game/blueprints/BatterySlot` (`/Game/blueprints/Battery.SlotID` _asbattery)))
          (set `/Game/blueprints/BatterySlot.BatterySlotOccupied` false _asbattery_slot_3)
          (set `self.IsHolding` true)
          (`/Game/blueprints/Battery.BatteryUnplugged` _asbattery)
          (`PrimitiveComponent.SetSimulatePhysics` _battery_2 false)
          (`PrimitiveComponent.SetRenderCustomDepth` _battery_2 false)
          (`PrimitiveComponent.SetCustomDepthStencilValue` _battery_2 0)
          (set `self.LookingAtSlot` false)
          (set `self.BatterySlot` null)
          (else
            (set `self.IsHolding` true)
            (`PrimitiveComponent.SetSimulatePhysics` _battery_3 false)
            (`PrimitiveComponent.SetRenderCustomDepth` _battery_3 false)
            (`PrimitiveComponent.SetCustomDepthStencilValue` _battery_3 0)))))))

(event `/Game/blueprints/player/crouch.Toggle Crouch`
  (params (IsCrouched :type Boolean))
  (if IsCrouched
    (bind (_direction _lerp) (`Timeline|Interpolation` :!label _label_8)
      (:`Update`
        (`CapsuleComponent.SetCapsuleHalfHeight` (`self.CapsuleComponent`) (`KismetMathLibrary.Lerp` 40.0 88.0 _lerp) true)))
    (else
      (goto _label_8 :!via `Reverse`))))

(event `Key|LeftControl`
  (params (Key :type "Key Structure"))
  (:`Pressed`
    (bind _isa (`/Engine/EditorBlueprintResources/StandardMacros.FlipFlop`)
      (:`A`
        _)
      (:`B`
        _))
    (`/Game/blueprints/player/crouch.Toggle Crouch` _isa)))

(fn `UserConstructionScript`)