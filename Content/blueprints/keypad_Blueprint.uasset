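; Keypad Blueprint that plays a scripted unlock sequence when ActionLaunched fires, with no check of an entered code.
; If locked, it reveals four code components one after another, turns the indicator material green and clears IsLocked.
; It then hides the code and, after a timed delay, automatically relocks with a red indicator.
; Firing ActionLaunched while unlocked relocks immediately through the same branch.
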(event `self.ActionLaunched`
  (params (`LaunchedFromDoor?` :type Boolean))
  (bind _keypad (`self.keypad`))
  (bind _code1 (`self.code1`))
  (bind _code2 (`self.code2`))
  (bind _code3 (`self.code3`))
  (bind _code4 (`self.code4`))
  (if (`self.isLocked?`)
    (`SceneComponent.SetVisibility` _code1 true false)
    (`KismetSystemLibrary.Delay` 0.2)
    (`SceneComponent.SetVisibility` _code2 true false)
    (`KismetSystemLibrary.Delay` 0.2)
    (`SceneComponent.SetVisibility` _code3 true false)
    (`KismetSystemLibrary.Delay` 0.2)
    (`SceneComponent.SetVisibility` _code4 true false)
    (`KismetSystemLibrary.Delay` 1.0)
    (`PrimitiveComponent.SetMaterial` _keypad 5 "/Game/Materials/IndicatorLightOn-green.IndicatorLightOn-green")
    (set `self.isLocked?` false)
    (`KismetSystemLibrary.Delay` 1.0)
    (`SceneComponent.SetVisibility` _code1 false false)
    (`SceneComponent.SetVisibility` _code2 false false)
    (`SceneComponent.SetVisibility` _code3 false false)
    (`SceneComponent.SetVisibility` _code4 false false)
    (`KismetSystemLibrary.Delay` 3.0)
    (`self.lockBackOn`)
    (else
      (set `self.isLocked?` true :!label _label)
      (`PrimitiveComponent.SetMaterial` _keypad 5 "/Game/Materials/IndicatorLightOn-red.IndicatorLightOn-red"))))

(event `lockBackOn`
  (goto _label))

(fn `UserConstructionScript`
  (`parent.UserConstructionScript`))