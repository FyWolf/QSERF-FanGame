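; Battery slot that links a battery to the Ship as slot 1 or 2.
; Overlap events show and hide a green holographic battery mesh.
; When occupied, it stores the reported charge, refreshes a dial and notifies the Ship, while level changes pass back to the connected battery.
; Plug, death and revive events route to the Ship's per-slot functions by SlotNumber.
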(event `BeginOverlap`
  (`SceneComponent.SetVisibility` (`self.battery`) true false)
  (`PrimitiveComponent.SetMaterial` (`self.battery`) 0 "/Game/Materials/HoloGreen.HoloGreen"))

(event `EndOverlap`
  (`SceneComponent.SetVisibility` (`self.battery`) false false)
  (`PrimitiveComponent.SetMaterial` (`self.battery`) 0 "/Game/Materials/HoloGreen.HoloGreen"))

(event `BatteryGatherLevel`
  (params (Charge :type "Float (double-precision)"))
  (bind _ship (`self.Ship`))
  (bind _slotnumber (`self.SlotNumber`))
  (if (`self.BatterySlotOccupied`)
    (bind _output_get (set `self.BatteryLevel` Charge))
    (`/Game/blueprints/Dial.Battery Update` (`self.DialBattery`) _output_get)
    (if (== _slotnumber 1)
      (`/Game/blueprints/Cockpit.Battery1LevelUpdate` _ship)
      (elif (== _slotnumber 2)
        (`/Game/blueprints/Cockpit.Battery2LevelUpdate` _ship)))))

(event `BatteryLevelUpdate`
  (params (Changes :type "Float (double-precision)"))
  (`/Game/blueprints/Battery.BatteryUdpate` (`self.ConnectedBattery`) Changes))

(event `BatteryPlugged`
  (params (IsPlugged :type Boolean) (Level :type "Float (double-precision)"))
  (bind _slotnumber (`self.SlotNumber`))
  (bind _ship (`self.Ship`))
  (if (== _slotnumber 1)
    (`/Game/blueprints/Cockpit.Battery1plugged` _ship IsPlugged)
    (elif (== _slotnumber 2)
      (`/Game/blueprints/Cockpit.Battery2Plugged` _ship IsPlugged))))

(event `BatteryDead`
  (bind _ship (`self.Ship`))
  (bind _slotnumber (`self.SlotNumber`))
  (if (== _slotnumber 1)
    (`/Game/blueprints/Cockpit.Battery1Death` _ship true)
    (elif (== _slotnumber 2)
      (`/Game/blueprints/Cockpit.Battery2Death` _ship true))))

(event `BatteryRevive`
  (bind _ship (`self.Ship`))
  (bind _slotnumber (`self.SlotNumber`))
  (if (== _slotnumber 1)
    (`/Game/blueprints/Cockpit.Battery1Death` _ship false)
    (elif (== _slotnumber 2)
      (`/Game/blueprints/Cockpit.Battery2Death` _ship false))))

(fn `UserConstructionScript`)