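; Security door Blueprint that swings its mesh open and closed on ActionLaunched, gated by a referenced keypad's lock.
; Unlocked, a FlipFlop plays or reverses a yaw Timeline, with swing direction set by OppeningSide.
; Locked, an open door closes, while a closed one plays a separate yaw animation without opening.
; Toggles and locked closes propagate to any paired door, using LaunchedFromDoor to prevent call loops.
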(event `self.ActionLaunched`
  (params (`LaunchedFromDoor?` :type Boolean))
  (bind _ispaired_ (`self.IsPaired?`))
  (bind _qsdoor_door_security (`self.QSDoor_door_security`))
  (if (`/Game/blueprints/keypad_Blueprint.isLocked?` (`self.refKeypad`))
    (if (`self.isOppened?`)
      (`|ExecutionSequence`
        (:`then_0`
          (if `LaunchedFromDoor?`
            _
            (elif _ispaired_
              (`self.ActionLaunched` (`self.PairedDoor`) true :!label _label))))
        (:`then_1`
          (set `self.isOppened?` false :!label _label_2)
          (bind (_direction _newtrack_0) (`Timeline|Timeline_0` :!via `Reverse` :!label _label_3)
            (:`Update`
              (if (`self.OppeningSide`)
                (`SceneComponent.K2_SetRelativeRotation` _qsdoor_door_security (`KismetMathLibrary.MakeRotator` 0.0 0.0 _newtrack_0) false false)
                (else
                  (`SceneComponent.K2_SetRelativeRotation` _qsdoor_door_security (`KismetMathLibrary.MakeRotator` 0.0 0.0 (* _newtrack_0 -1.0)) false false)))))))
      (else
        (bind (_direction_2 _newtrack_0_2) (`Timeline|Timeline_1` :!via `PlayFromStart`)
          (:`Update`
            (`SceneComponent.K2_SetRelativeRotation` (`self.QSDoor_door_security`) (`KismetMathLibrary.MakeRotator` 0.0 0.0 _newtrack_0_2) false false)))))
    (else
      (if `LaunchedFromDoor?`
        _
        (elif _ispaired_
          (`|ExecutionSequence`
            (:`then_0`
              (goto _label))
            (:`then_1`
              _))))
      (`/Engine/EditorBlueprintResources/StandardMacros.FlipFlop`
        (:`A`
          (set `self.isOppened?` true)
          (goto _label_3))
        (:`B`
          (goto _label_2))))))

(fn `UserConstructionScript`)