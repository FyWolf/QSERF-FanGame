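; Elevator Blueprint that slides a door mesh open and closed along its relative X axis each time ActionLaunched is called.
; A FlipFlop alternately plays and reverses a timeline whose track sets the door offset, negated when OppeningSide is set.
; When IsPaired, it first triggers PairedDoor with LaunchedFromDoor true, so both doors toggle together without calling each other back.
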(event `self.ActionLaunched`
  (params (`LaunchedFromDoor?` :type Boolean))
  (bind _qsdoor_door__window_1 (`self.QSDoor_door__window_1`))
  (if `LaunchedFromDoor?`
    (`/Engine/EditorBlueprintResources/StandardMacros.FlipFlop` :!label _label
      (:`A`
        (bind (_direction _newtrack_0) (`Timeline|Timeline_0` :!label _label_2)
          (:`Update`
            (if (`self.OppeningSide`)
              (`SceneComponent.K2_SetRelativeLocation` _qsdoor_door__window_1 (`KismetMathLibrary.MakeVector` (* _newtrack_0 -1.0)) false false)
              (else
                (`SceneComponent.K2_SetRelativeLocation` _qsdoor_door__window_1 (`KismetMathLibrary.MakeVector` _newtrack_0) false false))))))
      (:`B`
        (goto _label_2 :!via `Reverse`)))
    (elif (`self.IsPaired?`)
      (`|ExecutionSequence`
        (:`then_0`
          (`self.ActionLaunched` (`self.PairedDoor`) true))
        (:`then_1`
          (goto _label)))
      (else
        (goto _label)))))

(fn `UserConstructionScript`)