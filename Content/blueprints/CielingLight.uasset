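; Ceiling light actor for a ship that drains the ship's battery and shows normal, emergency and power-out states.
; Tick charges a smaller battery cost for emergency than normal lighting, and blinks the RectLight red and black while PowerOut is set.
; LightEmergency and LightNormal use randomized delays and loops for flicker transitions toward red or white.
; LightNoPowerStart sets PowerOut; the emergency and normal flags are only read here.
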(event `self.ReceiveTick`
  (params (DeltaSeconds :type "Float (single-precision)"))
  (bind _ship (`self.Ship`))
  (`|ExecutionSequence`
    (:`then_0`
      (if (`self.EmergencyLight`)
        (`/Game/blueprints/Cockpit.BatteryUpdate` _ship -0.001)
        (elif (`self.NormalLight`)
          (`/Game/blueprints/Cockpit.BatteryUpdate` _ship -0.003))))
    (:`then_1`
      (if (`self.PowerOut`)
        (`KismetSystemLibrary.Delay` (`KismetMathLibrary.FClamp` (`KismetMathLibrary.RandomFloat`) 0.5 1.3))
        (`LightComponent.SetLightColor` (`self.RectLight`) (struct :`R` 1.0 :`A` 1.0) true)
        (`KismetSystemLibrary.Delay` (`KismetMathLibrary.FClamp` (`KismetMathLibrary.RandomFloat`) 0.5 1.3))
        (`LightComponent.SetLightColor` (`self.RectLight`) (struct :`A` 1.0) true)))))

(event `Light Emergency`
  (for _ (range (+ (`KismetMathLibrary.RandomInteger` 10) 1))
    (`KismetSystemLibrary.Delay` (`KismetMathLibrary.FClamp` (`KismetMathLibrary.RandomFloat`) 0.1 0.5))
    (`LightComponent.SetLightColor` (`self.RectLight`) (struct :`R` 1.0 :`A` 1.0) true)
    (`KismetSystemLibrary.Delay` (`KismetMathLibrary.FClamp` (`KismetMathLibrary.RandomFloat`) 0.1 0.5))
    (`LightComponent.SetLightColor` (`self.RectLight`) (struct :`A` 1.0) true))
  (`KismetSystemLibrary.Delay` (`KismetMathLibrary.FClamp` (`KismetMathLibrary.RandomFloat`) 1.2 1.5))
  (`LightComponent.SetLightColor` (`self.RectLight`) (struct :`R` 1.0 :`A` 1.0) true))

(event `LightNormal`
  (for _ (range (+ (`KismetMathLibrary.RandomInteger` 10) 1))
    (`KismetSystemLibrary.Delay` (`KismetMathLibrary.FClamp` (`KismetMathLibrary.RandomFloat`) 0.1 0.5))
    (`LightComponent.SetLightColor` (`self.RectLight`) (struct :`R` 1.0 :`G` 1.0 :`B` 1.0 :`A` 1.0) true)
    (`KismetSystemLibrary.Delay` (`KismetMathLibrary.FClamp` (`KismetMathLibrary.RandomFloat`) 0.1 0.5))
    (`LightComponent.SetLightColor` (`self.RectLight`) (struct :`A` 1.0) true))
  (`KismetSystemLibrary.Delay` (`KismetMathLibrary.FClamp` (`KismetMathLibrary.RandomFloat`) 1.2 1.5))
  (`LightComponent.SetLightColor` (`self.RectLight`) (struct :`R` 1.0 :`G` 1.0 :`B` 1.0 :`A` 1.0) true))

(event `LightNoPowerStart`
  (params (OutOfPower :type Boolean))
  (set `self.PowerOut` OutOfPower))

(fn `UserConstructionScript`)