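; Red light Blueprint that an interaction signal switches on or off, powered by the ship's first battery.
; Switching toggles the point light and swaps the indicator material, and only works while CanWork is true.
; While on, it drains Battery 1 by a fixed amount every Tick, independent of delta time.
; BatteryDead sets CanWork, and Tick keeps the light forced off while the battery is dead.
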(event `self.On Interraction`
  (params (BoolSignal :type Boolean))
  (bind _indicator (`self.indicator`))
  (if (`self.CanWork`)
    (`SceneComponent.SetVisibility` (`self.PointLight`) BoolSignal false)
    (if BoolSignal
      (`PrimitiveComponent.SetMaterial` _indicator 1 "/Game/Materials/IndicatorLightOn-red.IndicatorLightOn-red")
      (set `self.IsOn` true)
      (else
        (`PrimitiveComponent.SetMaterial` _indicator 1 "/Game/Materials/IndicatorLightOff.IndicatorLightOff")
        (set `self.IsOn` false)))))

(event `self.ReceiveTick`
  (params (DeltaSeconds :type "Float (single-precision)"))
  (`|ExecutionSequence`
    (:`then_0`
      (if (not (`self.CanWork`))
        (`SceneComponent.SetVisibility` (`self.PointLight`) false false)
        (`PrimitiveComponent.SetMaterial` (`self.indicator`) 1 "/Game/Materials/IndicatorLightOff.IndicatorLightOff")
        (set `self.IsOn` false)))
    (:`then_1`
      (if (`self.IsOn`)
        (`/Game/blueprints/Cockpit.Battery1LevelUpdate` (`self.Ship`) -0.001)))))

(event `self.BatteryDead`
  (params (IsBatteryDead :type Boolean))
  (set `self.CanWork` (not IsBatteryDead)))

(fn `UserConstructionScript`
  (`parent.UserConstructionScript`))