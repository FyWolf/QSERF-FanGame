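; Server prop Blueprint with a toggleable power state and a sliding Server component.
; Power events swap the indicator light material and set ServerOn, which makes Tick spin four fan cylinders.
; The position toggle alternately plays and reverses a timeline that offsets the Server along its forward vector.
; That offset builds on the relative location cached at BeginPlay but is applied as a world location.
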(event `self.ReceiveTick`
  (params (DeltaSeconds :type "Float (single-precision)"))
  (if (`self.serverOn`)
    (`SceneComponent.K2_AddRelativeRotation` (`self.serverFan_Cylinder9`) (struct :`Roll` 20.0) false false)
    (`SceneComponent.K2_AddRelativeRotation` (`self.serverFan_Cylinder7`) (struct :`Roll` 20.0) false false)
    (`SceneComponent.K2_AddRelativeRotation` (`self.serverFan_Cylinder5`) (struct :`Roll` 20.0) false false)
    (`SceneComponent.K2_AddRelativeRotation` (`self.serverFan_Cylinder`) (struct :`Roll` 20.0) false false)))

(event `self.ReceiveBeginPlay`
  (set `self.NewVar_0` (`SceneComponent.RelativeLocation` (`self.Server`))))

(event `ServerTogglePosition`
  (bind _server (`self.Server`))
  (`/Engine/EditorBlueprintResources/StandardMacros.FlipFlop`
    (:`A`
      (bind (_direction _lerp) (`Timeline|Timeline_0` :!label _label)
        (:`Update`
          (bind _returnvalue (`KismetMathLibrary.Lerp` 100.0 0.0 _lerp))
          (`SceneComponent.K2_SetWorldLocation` _server (+ (`self.NewVar_0`) (* (`SceneComponent.GetForwardVector` _server) (`KismetMathLibrary.MakeVector` _returnvalue _returnvalue _returnvalue))) false false))))
    (:`B`
      (goto _label :!via `Reverse`))))

(event `ServerPowerOn`
  (`PrimitiveComponent.SetMaterial` (`self.Server`) 1 "/Game/Materials/IndicatorLightOn-green.IndicatorLightOn-green")
  (set `self.serverOn` true))

(event `ServerPowerOff`
  (`PrimitiveComponent.SetMaterial` (`self.Server`) 1 "/Game/Materials/IndicatorLightOff.IndicatorLightOff")
  (set `self.serverOn` false))

(fn `UserConstructionScript`)