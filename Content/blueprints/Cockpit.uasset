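; Cockpit actor that runs a ship's two-slot battery power, its lights and the battery indicators.
; Tick drives the lights' no-power state and, through short delays and cross-resetting DoOnce nodes, each indicator's normal, low or down state.
; The light button flips between normal and emergency lighting, and plug events re-evaluate it, blacking out when both slots are empty.
; BatteryUpdate applies charge changes to battery one, falling back to battery two when it is unplugged or dead.
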(event `self.ReceiveTick`
  (params (DeltaSeconds :type "Float (single-precision)"))
  (bind _battery1indicator (`self.Battery1Indicator`))
  (bind _battery2indicator (`self.Battery2Indicator`))
  (bind _battery1level (`self.Battery1Level`))
  (bind _battery2level (`self.Battery2Level`))
  (bind _shiplights (`self.ShipLights`))
  (`|ExecutionSequence`
    (:`then_0`
      (if (and (not (`self.Batery2`)) (not (`self.Battery1`)))
        (for _array_element _shiplights
          (`/Game/blueprints/CielingLight.LightNoPowerStart` _array_element false))
        (else
          (for _array_element_2 _shiplights
            (`/Game/blueprints/CielingLight.LightNoPowerStart` _array_element_2 (or (and (not (`self.Batery2`)) (`self.Battery1Dead`)) (and (not (`self.Battery1`)) (`self.Battery2Dead`)) (and (`self.Battery1Dead`) (`self.Battery2Dead`))))))))
    (:`then_1`
      (if (`self.Battery1`)
        (`KismetSystemLibrary.Delay` 0.2)
        (if (< _battery1level 0.5)
          (if (< _battery1level 0.2)
            (`/Game/blueprints/Indicator_Master.BatteryDown` _battery1indicator true)
            (`/Engine/EditorBlueprintResources/StandardMacros.DoOnce` false :!label _label
              (:`Completed`
                (`/Game/blueprints/Indicator_Master.BatteryLow` _battery1indicator false)
                (`/Game/blueprints/Indicator_Master.On Interraction` _battery1indicator false)
                (`|ExecutionSequence`
                  (:`then_0`
                    (goto _label_2 :!via `Reset`))
                  (:`then_1`
                    (goto _label_3 :!via `Reset`)))))
            (else
              (`/Game/blueprints/Indicator_Master.BatteryLow` _battery1indicator true)
              (`/Engine/EditorBlueprintResources/StandardMacros.DoOnce` false :!label _label_2
                (:`Completed`
                  (`/Game/blueprints/Indicator_Master.BatteryDown` _battery1indicator false)
                  (`/Game/blueprints/Indicator_Master.On Interraction` _battery1indicator false)
                  (`|ExecutionSequence`
                    (:`then_0`
                      (goto _label :!via `Reset`))
                    (:`then_1`
                      (goto _label_3 :!via `Reset`)))))))
          (else
            (`/Game/blueprints/Indicator_Master.On Interraction` _battery1indicator true)
            (`/Engine/EditorBlueprintResources/StandardMacros.DoOnce` false :!label _label_3
              (:`Completed`
                (`/Game/blueprints/Indicator_Master.BatteryDown` _battery1indicator false)
                (`/Game/blueprints/Indicator_Master.BatteryLow` _battery1indicator false)
                (`|ExecutionSequence`
                  (:`then_0`
                    (goto _label_2 :!via `Reset`))
                  (:`then_1`
                    (goto _label :!via `Reset`)))))))))
    (:`then_2`
      (if (`self.Batery2`)
        (`KismetSystemLibrary.Delay` 0.2)
        (if (< _battery2level 0.5)
          (if (< _battery2level 0.2)
            (`/Game/blueprints/Indicator_Master.BatteryDown` _battery2indicator true)
            (`/Engine/EditorBlueprintResources/StandardMacros.DoOnce` false :!label _label_4
              (:`Completed`
                (`/Game/blueprints/Indicator_Master.BatteryLow` _battery2indicator false)
                (`/Game/blueprints/Indicator_Master.On Interraction` _battery2indicator false)
                (`|ExecutionSequence`
                  (:`then_0`
                    (goto _label_5 :!via `Reset`))
                  (:`then_1`
                    (goto _label_6 :!via `Reset`)))))
            (else
              (`/Game/blueprints/Indicator_Master.BatteryLow` _battery2indicator true)
              (`/Engine/EditorBlueprintResources/StandardMacros.DoOnce` false :!label _label_5
                (:`Completed`
                  (`/Game/blueprints/Indicator_Master.BatteryDown` _battery2indicator false)
                  (`/Game/blueprints/Indicator_Master.On Interraction` _battery2indicator false)
                  (`|ExecutionSequence`
                    (:`then_0`
                      (goto _label_4 :!via `Reset`))
                    (:`then_1`
                      (goto _label_6 :!via `Reset`)))))))
          (else
            (`/Game/blueprints/Indicator_Master.On Interraction` _battery2indicator true)
            (`/Engine/EditorBlueprintResources/StandardMacros.DoOnce` false :!label _label_6
              (:`Completed`
                (`/Game/blueprints/Indicator_Master.BatteryDown` _battery2indicator false)
                (`/Game/blueprints/Indicator_Master.BatteryLow` _battery2indicator false)
                (`|ExecutionSequence`
                  (:`then_0`
                    (goto _label_5 :!via `Reset`))
                  (:`then_1`
                    (goto _label_4 :!via `Reset`)))))))))))

(event `self.ReceiveBeginPlay`
  (for _array_element (`self.BatterySlot`)
    (set `/Game/blueprints/BatterySlot.Ship` self _array_element)))

(event `LightButton`
  (bind _shiplights (`self.ShipLights`))
  (bind _isa (`/Engine/EditorBlueprintResources/StandardMacros.FlipFlop`)
    (:`A`
      (set `self.Light on` _isa))
    (:`B`
      (set `self.Light on` _isa)))
  (if (or (and (not (`self.Batery2`)) (`self.Battery1Dead`)) (and (not (`self.Battery1`)) (`self.Battery2Dead`)) (and (`self.Battery1Dead`) (`self.Battery2Dead`))) :!label _label_7
    _
    (elif (or (`self.Battery1`) (`self.Batery2`))
      (if (`self.Light on`)
        (for _array_element _shiplights
          (if (not (`/Game/blueprints/CielingLight.NormalLight` _array_element))
            (`/Game/blueprints/CielingLight.LightNormal` _array_element)
            (set `/Game/blueprints/CielingLight.NormalLight` true _array_element)
            (set `/Game/blueprints/CielingLight.EmergencyLight` false _array_element)
            (`/Game/blueprints/CielingLight.LightNoPowerStart` _array_element false)))
        (else
          (for _array_element_2 _shiplights
            (if (not (`/Game/blueprints/CielingLight.EmergencyLight` _array_element_2))
              (`/Game/blueprints/CielingLight.Light Emergency` _array_element_2)
              (set `/Game/blueprints/CielingLight.EmergencyLight` true _array_element_2)
              (set `/Game/blueprints/CielingLight.NormalLight` false _array_element_2)
              (`/Game/blueprints/CielingLight.LightNoPowerStart` _array_element_2 false)))))
      (else
        (for _array_element_3 _shiplights
          (`LightComponent.SetLightColor` (`/Game/blueprints/CielingLight.RectLight` _array_element_3) (struct :`A` 1.0) true)
          (set `/Game/blueprints/CielingLight.EmergencyLight` false _array_element_3)
          (set `/Game/blueprints/CielingLight.NormalLight` false _array_element_3)
          (`/Game/blueprints/CielingLight.LightNoPowerStart` _array_element_3 false))))))

(event `Battery1plugged`
  (params (IsPlugged :type Boolean))
  (bind _battery1indicator (`self.Battery1Indicator`))
  (bind _output_get (set `self.Battery1` IsPlugged))
  (`/Game/blueprints/Indicator_Master.On Interraction` _battery1indicator _output_get)
  (`/Game/blueprints/Indicator_Master.BatteryDown` _battery1indicator false)
  (`/Game/blueprints/Indicator_Master.BatteryLow` _battery1indicator false)
  (goto _label_7))

(event `Battery2Plugged`
  (params (IsPlugged :type Boolean))
  (bind _battery2indicator (`self.Battery2Indicator`))
  (bind _output_get (set `self.Batery2` IsPlugged))
  (`/Game/blueprints/Indicator_Master.On Interraction` _battery2indicator _output_get)
  (`/Game/blueprints/Indicator_Master.BatteryDown` _battery2indicator false)
  (`/Game/blueprints/Indicator_Master.BatteryLow` _battery2indicator false)
  (goto _label_7))

(event `Battery1LevelUpdate`
  (set `self.Battery1Level` (`/Game/blueprints/BatterySlot.BatteryLevel` (`|GetArrayItem` (`self.BatterySlot`)))))

(event `Battery2LevelUpdate`
  (set `self.Battery2Level` (`/Game/blueprints/BatterySlot.BatteryLevel` (`|GetArrayItem` (`self.BatterySlot`) 1))))

(event `Battery1Death`
  (params (state :type Boolean))
  (set `self.Battery1Dead` state))

(event `Battery2Death`
  (params (State :type Boolean))
  (set `self.Battery2Dead` State))

(event `BatteryUpdate`
  (params (Ammount :type "Float (double-precision)"))
  (if (`self.Battery1`)
    (if (`self.Battery1Dead`)
      (if (`self.Batery2`) :!label _label_8
        (if (not (`self.Battery2Dead`))
          (`/Game/blueprints/BatterySlot.BatteryLevelUpdate` (`|GetArrayItem` (`self.BatterySlot`) 1) Ammount)))
      (else
        (`/Game/blueprints/BatterySlot.BatteryLevelUpdate` (`|GetArrayItem` (`self.BatterySlot`)) Ammount)))
    (else
      (goto _label_8))))

(fn `UserConstructionScript`)